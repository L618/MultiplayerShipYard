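; Battle royale plane actor that flies across the map and supplies spawn points for players.
; E_StartMoving sets a fixed velocity along X on its ProjectileMovement component to start the flight.
; FSGetPlayerSpawnLocation returns the PlayersSpawnLocation component's world position with a small positive random offset on each axis, scattering the returned positions.
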(event `E_StartMoving`
  (set `MovementComponent.Velocity` (600.0 0.0 0.0) (`self.ProjectileMovement`)))

(fn `FS_GetPlayerSpawnLocation`
  (returns (SpawnLocation :type "Vector Structure"))
  (bind _returnvalue (`KismetMathLibrary.RandomFloatInRange` 0.0 200.0))
  (bind _returnvalue_2 (`SceneComponent.K2_GetComponentToWorld` (`self.PlayersSpawnLocation`)))
  (return (`KismetMathLibrary.MakeVector` (+ (.x (.location _returnvalue_2)) _returnvalue) (+ (.y (.location _returnvalue_2)) _returnvalue) (+ (.z (.location _returnvalue_2)) _returnvalue))))

(fn `UserConstructionScript`)