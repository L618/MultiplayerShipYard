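; Battle royale barrier that shrinks the safe zone in stages and applies periodic damage to BR_Characters outside it.
; Authority-gated start and stop events alternate a one-second countdown timer with movement until the final scale is reached.
; While moving, Tick interpolates DamageZone's scale toward half its previous X and Y, keeping Z.
; Leaving DamageZone starts permanent damage on the character's HealthComponent, and re-entering stops it.
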(event `self.ReceiveBeginPlay`
  (set `self.DamageZoneScaleBeforeLastReduction` (`SceneComponent.RelativeScale3D` (`self.DamageZone`))))

(event `EA_StartBarrierMoving`
  (params (IsGameStart :type Boolean))
  ;[1 1 1] Reduce barrier to the certain size. Last size - "x = 5, y = 5, z = 50"
  (`/Engine/EditorBlueprintResources/ActorMacros.Switch Has Authority`
    (:`Authority`
      (if IsGameStart
        (`self.FS_StartPauseTimer`)
        (elif (not (== (`self.DamageZoneScaleBeforeLastReduction`) (`self.LastScale`) :`ErrorTolerance` 5.0))
          (set `self.IsMoving` true))))))

(event `EA_StopBarrierMoving`
  ;[1 1 1] Stop barrier moving and start again after "delayBetweenBarrierMove" time
  (`/Engine/EditorBlueprintResources/ActorMacros.Switch Has Authority`
    (:`Authority`
      (set `self.IsMoving` false)
      (`self.FS_StartPauseTimer`))))

(event `self.ReceiveTick`
  (params (DeltaSeconds :type "Float (single-precision)"))
  ;[1 1 1] reduce barrier size
  (if (`self.IsMoving`)
    (`self.FS_ReduceSize`)))

(event `self.DamageZone.OnComponentBeginOverlap`
  (params (OverlappedComponent :type "PrimitiveComponent Object Reference") (OtherActor :type "Actor Object Reference") (OtherComp :type "PrimitiveComponent Object Reference") (OtherBodyIndex :type Integer) (bFromSweep :type Boolean) (SweepResult :type "HitResult Structure (by ref)"))
  (bind _asbr_character (cast `/Game/RPMSF/Blueprints/CustomCharacters/BR_Character` OtherActor))
  (`/Game/RPMSF/Blueprints/Kernel_Character/Components/HealthComponent.FS_StopPermanentDamage` (`/Game/RPMSF/Blueprints/Kernel_Character/CoreCharacter.HealthComponent` _asbr_character)))

(event `self.DamageZone.OnComponentEndOverlap`
  (params (OverlappedComponent :type "PrimitiveComponent Object Reference") (OtherActor :type "Actor Object Reference") (OtherComp :type "PrimitiveComponent Object Reference") (OtherBodyIndex :type Integer))
  (bind _asbr_character (cast `/Game/RPMSF/Blueprints/CustomCharacters/BR_Character` OtherActor))
  (`/Game/RPMSF/Blueprints/Kernel_Character/Components/HealthComponent.FS_StartPermanentDamage` (`/Game/RPMSF/Blueprints/Kernel_Character/CoreCharacter.HealthComponent` _asbr_character) 1.0 0.5))

(fn `FS_PauseTimer`
  (bind _output_get (set `self.CurrentTime` (- (`self.CurrentTime`) 1)))
  (if (<= _output_get 0)
    (`self.FS_StopPauseTimer`)
    (`self.EA_StartBarrierMoving` false)))

(fn `FS_ReduceSize`
  (bind _returnvalue (`KismetMathLibrary.VInterpTo` (`SceneComponent.RelativeScale3D` (`self.DamageZone`)) (/ (`self.DamageZoneScaleBeforeLastReduction`) (2.0 2.0 1.0)) (`GameplayStatics.GetWorldDeltaSeconds`) 0.1))
  (`SceneComponent.SetRelativeScale3D` (`self.DamageZone`) _returnvalue)
  (if (== _returnvalue (/ (`self.DamageZoneScaleBeforeLastReduction`) (2.0 2.0 1.0)) :`ErrorTolerance` 1.0)
    (set `self.DamageZoneScaleBeforeLastReduction` _returnvalue)
    (`self.EA_StopBarrierMoving`)))

(fn `FS_StartPauseTimer`
  (set `self.CurrentTime` (`self.DelayBetweenMovesTime`))
  (bind _returnvalue (`KismetSystemLibrary.K2_SetTimer` null "FS_PauseTimer" 1.0 true))
  (set `self.PauseTimer` _returnvalue))

(fn `FS_StopPauseTimer`
  (`KismetSystemLibrary.K2_ClearAndInvalidateTimerHandle` (`self.PauseTimer`)))

(fn `UserConstructionScript`)