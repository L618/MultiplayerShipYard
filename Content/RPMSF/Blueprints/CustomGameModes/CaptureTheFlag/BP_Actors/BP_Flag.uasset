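; BP_Flag is a team-colored Capture the Flag flag that tracks whether it is at base, carried or dropped.
; A server-only overlap lets enemies attach it to their mesh and lets teammates return it when dropped, updating the player state and notifying the team.
; Events return it to its base or drop it near the carrier, re-enabling collision.
; The color is applied after a delay that waits for team replication.
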(event `self.ReceiveBeginPlay`
  (set `self.FlagLocation` "NewEnumerator0")
  (`PrimitiveComponent.SetCollisionEnabled` (`self.Collision`) "QueryOnly")
  ;[1 1 1 1 15] to insure that team variable was replicated
  (`KismetSystemLibrary.Delay` 3.0)
  (bind _returnvalue (`PrimitiveComponent.CreateDynamicMaterialInstance` (`self.Flag`) 0 "/Game/RPMSF/Blueprints/CustomGameModes/CaptureTheFlag/BP_Actors/FlagMaterial.FlagMaterial"))
  (switch `int` (`self.Team`)
    (:`0`
      (`MaterialInstanceDynamic.SetVectorParameterValue` _returnvalue "Color" (struct :`R` 1.0 :`A` 1.0)))
    (:`1`
      (`MaterialInstanceDynamic.SetVectorParameterValue` _returnvalue "Color" (struct :`R` 0.034151 :`B` 1.0 :`A` 1.0)))))

(event `EA_ReturnFlagToTheBase`
  (bind _carriercharacter (`self.CarrierCharacter`))
  (bind _carriercharacter_2 (`self.CarrierCharacter`))
  (`self.K2_DetachFromActor` "KeepWorld" "KeepWorld" "KeepWorld")
  (`self.K2_SetActorTransform` (`SceneComponent.K2_GetComponentToWorld` (`/Game/RPMSF/Blueprints/CustomGameModes/CaptureTheFlag/BP_Actors/BP_FlagBase.FlagSpawnLocation` (`self.FlagBase`))))
  (`|ExecutionSequence`
    (:`then_0`
      (`/Engine/EditorBlueprintResources/StandardMacros.IsValid` _carriercharacter_2
        (:`Is Valid`
          (set `/Game/RPMSF/Blueprints/CustomCharacters/CTF_Character.Flag` null _carriercharacter_2))))
    (:`then_1`
      (`/Engine/EditorBlueprintResources/StandardMacros.IsValid` _carriercharacter
        (:`Is Valid`
          (bind _asctf_ps (cast `/Game/RPMSF/Blueprints/CustomGameModes/CaptureTheFlag/CTF_PS` (`Pawn.PlayerState` _carriercharacter)))
          (set `/Game/RPMSF/Blueprints/CustomGameModes/CaptureTheFlag/CTF_PS.HasFlag` false _asctf_ps))))
    (:`then_2`
      (set `self.CarrierCharacter` null))
    (:`then_3`
      (set `self.FlagLocation` "NewEnumerator0")
      (`PrimitiveComponent.SetCollisionEnabled` (`self.Collision`) "QueryOnly"))))

(event `EA_DropFlag`
  (`self.K2_SetActorLocation` (+ (`self.K2_GetActorLocation` (`self.CarrierCharacter`)) (`KismetMathLibrary.MakeVector` (`KismetMathLibrary.RandomFloatInRange` 40.0 70.0) (`KismetMathLibrary.RandomFloatInRange` 40.0 70.0) -90.0)))
  (`self.K2_SetActorRotation` (struct))
  (`self.K2_DetachFromActor` "KeepWorld" "KeepWorld" "KeepWorld")
  (set `self.FlagLocation` "NewEnumerator1")
  (set `self.CarrierCharacter` null)
  (`PrimitiveComponent.SetCollisionEnabled` (`self.Collision`) "QueryOnly"))

(event `self.Collision.OnComponentBeginOverlap`
  (params (OverlappedComponent :type "PrimitiveComponent Object Reference") (OtherActor :type "Actor Object Reference") (OtherComp :type "PrimitiveComponent Object Reference") (OtherBodyIndex :type Integer) (bFromSweep :type Boolean) (SweepResult :type "HitResult Structure (by ref)"))
  (`/Engine/EditorBlueprintResources/ActorMacros.Switch Has Authority`
    (:`Authority`
      (if (`|EnumInequality` (`self.FlagLocation`) "NewEnumerator2")
        (`self.FS_DecideWhatToDoWithFlag` OtherActor)))))

(fn `FS_DecideWhatToDoWithFlag`
  (params (OverlapActor :type "Actor Object Reference"))
  (locals (OverlapingChar :type "/Game/RPMSF/Blueprints/CustomCharacters/CTF_Character Object Reference") (CharPS :type "/Game/RPMSF/Blueprints/CustomGameModes/CaptureTheFlag/CTF_PS Object Reference") (NotifyTeam :type Integer))
  (bind _asctf_character (cast `/Game/RPMSF/Blueprints/CustomCharacters/CTF_Character` OverlapActor))
  (bind _output_get (set `local.OverlapingChar` _asctf_character))
  (bind _asctf_ps (cast `/Game/RPMSF/Blueprints/CustomGameModes/CaptureTheFlag/CTF_PS` (`Pawn.PlayerState` _output_get)))
  (set `local.CharPS` _asctf_ps)
  (switch `/Game/RPMSF/Blueprints/CustomGameModes/CaptureTheFlag/Enums/E_FlagLocation` (`self.FlagLocation`)
    (:`NewEnumerator0`
      _)
    (:`NewEnumerator1`
      _))
  (if (!= (`/Game/RPMSF/Blueprints/Kernel/CoreClasses/Core_PS.Team` (`local.CharPS`)) (`self.Team`))
    (if (`|EnumInequality` (`self.FlagLocation`) "NewEnumerator2")
      ;[1 1 1] do not delete
      (`PrimitiveComponent.SetCollisionEnabled` (`self.Collision`) "NoCollision")
      (set `/Game/RPMSF/Blueprints/CustomGameModes/CaptureTheFlag/CTF_PS.HasFlag` true (`local.CharPS`))
      (`self.K2_AttachToComponent` (`Character.Mesh` (`local.OverlapingChar`)) "pw1" "SnapToTarget" "SnapToTarget" "SnapToTarget" false)
      (set `self.FlagLocation` "NewEnumerator2")
      (bind _output_get_2 (set `self.CarrierCharacter` (`local.OverlapingChar`)))
      (set `/Game/RPMSF/Blueprints/CustomCharacters/CTF_Character.Flag` self _output_get_2)
      (`|ExecutionSequence`
        (:`then_0`
          (switch `int` (`/Game/RPMSF/Blueprints/Kernel/CoreClasses/Core_PS.Team` (`local.CharPS`))
            (:`0`
              (set `local.NotifyTeam` 1))
            (:`1`
              (set `local.NotifyTeam` 0))))
        (:`then_1`
          (`/Game/RPMSF/Blueprints/Kernel/CoreClasses/Core_GS.MC_SendNotification` (`/Game/RPMSF/Blueprints/Kernel/Helpers.H_GetCoreGS`) "Enemy has stolen our flag" false (`local.NotifyTeam`)))))
    (elif (`|EnumEquality` (`self.FlagLocation`) "NewEnumerator1")
      (`self.EA_ReturnFlagToTheBase`)
      (`/Game/RPMSF/Blueprints/Kernel/CoreClasses/Core_GS.MC_SendNotification` (`/Game/RPMSF/Blueprints/Kernel/Helpers.H_GetCoreGS`) "Flag has been returned to our base" false (`/Game/RPMSF/Blueprints/Kernel/CoreClasses/Core_PS.Team` (`local.CharPS`))))))

(fn `UserConstructionScript`)