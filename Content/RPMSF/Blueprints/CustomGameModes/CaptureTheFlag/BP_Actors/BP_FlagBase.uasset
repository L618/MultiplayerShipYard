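; Team flag base for the Capture The Flag mode, which spawns its flag and scores captures.
; On BeginPlay the server spawns a BP_Flag at the spawn point, passing its team and itself.
; When a same-team player carrying a flag overlaps the box, the server returns that flag, updates the team score via the game state and multicasts a notification.
; The capture check does not test whether the base's own flag is home.
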(event `self.ReceiveBeginPlay`
  (`/Engine/EditorBlueprintResources/ActorMacros.Switch Has Authority`
    (:`Authority`
      (`self.EA_CreateFlag`))))

(event `EA_CreateFlag`
  (`|SpawnActorFromClass` "/Game/RPMSF/Blueprints/CustomGameModes/CaptureTheFlag/BP_Actors/BP_Flag.BP_Flag_C" (`SceneComponent.K2_GetComponentToWorld` (`self.FlagSpawnLocation`)) "Undefined" "OverrideRootScale" null (`self.Team`) self null))

(event `self.BoxCollision.OnComponentBeginOverlap`
  (params (OverlappedComponent :type "PrimitiveComponent Object Reference") (OtherActor :type "Actor Object Reference") (OtherComp :type "PrimitiveComponent Object Reference") (OtherBodyIndex :type Integer) (bFromSweep :type Boolean) (SweepResult :type "HitResult Structure (by ref)"))
  (`/Engine/EditorBlueprintResources/ActorMacros.Switch Has Authority`
    (:`Authority`
      (bind _asctf_character (cast `/Game/RPMSF/Blueprints/CustomCharacters/CTF_Character` OtherActor))
      (bind _asctf_ps (cast `/Game/RPMSF/Blueprints/CustomGameModes/CaptureTheFlag/CTF_PS` (`Pawn.PlayerState` _asctf_character)))
      (bind _team (`/Game/RPMSF/Blueprints/Kernel/CoreClasses/Core_PS.Team` _asctf_ps))
      (bind _flag (`/Game/RPMSF/Blueprints/CustomCharacters/CTF_Character.Flag` _asctf_character))
      (if (and (== (`self.Team`) _team) (`/Game/RPMSF/Blueprints/CustomGameModes/CaptureTheFlag/CTF_PS.HasFlag` _asctf_ps) (`KismetSystemLibrary.IsValid` _flag))
        (`/Game/RPMSF/Blueprints/CustomGameModes/CaptureTheFlag/BP_Actors/BP_Flag.EA_ReturnFlagToTheBase` _flag)
        (`/Game/RPMSF/Blueprints/Kernel/CoreClasses/Core_GS.FS_UpdateTeamScore` (`/Game/RPMSF/Blueprints/Kernel/Helpers.H_GetCoreGS`) _team 0)
        (`|ExecutionSequence`
          (:`then_0`
            (switch `int` _team
              (:`0`
                (set `self.NotificationMessage` "RED TEAM has captured the enemy flag and got 1 score "))
              (:`1`
                (set `self.NotificationMessage` "BLUE TEAM has captured the enemy flag and got 1 score "))))
          (:`then_1`
            (`/Game/RPMSF/Blueprints/Kernel/CoreClasses/Core_GS.MC_SendNotification` (`/Game/RPMSF/Blueprints/Kernel/Helpers.H_GetCoreGS`) (`self.NotificationMessage`) true 0)))))))

(fn `UserConstructionScript`)