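; Main menu HUD that owns the front-end screens: main, multiplayer, host game and server browser menus.
; On BeginPlay it opens the main menu and shows the mouse cursor.
; Each screen has a toggle function that lazily creates and caches its widget, adds it to the viewport only if not already visible, and removes it from its parent to hide it.
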(event `self.ReceiveBeginPlay`
  (`self.F_ToggleMainMenu` true)
  (set `PlayerController.bShowMouseCursor` true (`self.PlayerOwner`)))

(fn `F_ToggleHostGameMenu`
  (params (Show :type Boolean))
  (bind _hostgamemenu (`self.HostGameMenu`))
  (if Show
    (`self.HostGameMenu`
      (:`then`
        (`/Game/RPMSF/Blueprints/Kernel/MacroHelpers.M_IsWidgetVisible` _hostgamemenu
          (:`false`
            (`UserWidget.AddToViewport` _hostgamemenu 0))))
      (:`else`
        (bind _returnvalue (`|CreateWidget` "/Game/RPMSF/UI/MainMenu/W_HostGameMenu.W_HostGameMenu_C" (`self.PlayerOwner`)))
        (bind _output_get (set `self.HostGameMenu` _returnvalue))
        (`UserWidget.AddToViewport` _output_get 0)))
    (else
      (bind _hostgamemenu_2 (`self.HostGameMenu`)
        (:`then`
          (`Widget.RemoveFromParent` _hostgamemenu_2))
        (:`else`)))))

(fn `F_ToggleMainMenu`
  (params (Show :type Boolean))
  (bind _mainmenuwb (`self.MainMenuWB`))
  (if Show
    (`self.MainMenuWB`
      (:`then`
        (`/Game/RPMSF/Blueprints/Kernel/MacroHelpers.M_IsWidgetVisible` _mainmenuwb
          (:`false`
            (`UserWidget.AddToViewport` _mainmenuwb 0))))
      (:`else`
        (bind _returnvalue (`|CreateWidget` "/Game/RPMSF/UI/MainMenu/W_MainMenu.W_MainMenu_C" (`self.PlayerOwner`)))
        (bind _output_get (set `self.MainMenuWB` _returnvalue))
        (`UserWidget.AddToViewport` _output_get 0)))
    (else
      (bind _mainmenuwb_2 (`self.MainMenuWB`)
        (:`then`
          (`Widget.RemoveFromParent` _mainmenuwb_2))
        (:`else`)))))

(fn `F_ToggleMultiplayerMenu`
  (params (Show :type Boolean))
  (bind _multiplayermenub (`self.MultiplayerMenuB`))
  (if Show
    (`self.MultiplayerMenuB`
      (:`then`
        (`/Game/RPMSF/Blueprints/Kernel/MacroHelpers.M_IsWidgetVisible` _multiplayermenub
          (:`false`
            (`UserWidget.AddToViewport` _multiplayermenub 0))))
      (:`else`
        (bind _returnvalue (`|CreateWidget` "/Game/RPMSF/UI/MainMenu/W_MultiplayerMenu.W_MultiplayerMenu_C" (`self.PlayerOwner`)))
        (bind _output_get (set `self.MultiplayerMenuB` _returnvalue))
        (`UserWidget.AddToViewport` _output_get 0)))
    (else
      (bind _multiplayermenub_2 (`self.MultiplayerMenuB`)
        (:`then`
          (`Widget.RemoveFromParent` _multiplayermenub_2))
        (:`else`)))))

(fn `F_ToggleServerBrowserMenu`
  (params (Show :type Boolean))
  (bind _serverbrowsermenuwb (`self.ServerBrowserMenuWB`))
  (if Show
    (`self.ServerBrowserMenuWB`
      (:`then`
        (`/Game/RPMSF/Blueprints/Kernel/MacroHelpers.M_IsWidgetVisible` _serverbrowsermenuwb
          (:`false`
            (`UserWidget.AddToViewport` _serverbrowsermenuwb 0))))
      (:`else`
        (bind _returnvalue (`|CreateWidget` "/Game/RPMSF/UI/MainMenu/W_ServerBrowserMenu.W_ServerBrowserMenu_C" (`self.PlayerOwner`)))
        (bind _output_get (set `self.ServerBrowserMenuWB` _returnvalue))
        (`UserWidget.AddToViewport` _output_get 0)))
    (else
      (bind _serverbrowsermenuwb_2 (`self.ServerBrowserMenuWB`)
        (:`then`
          (`Widget.RemoveFromParent` _serverbrowsermenuwb_2))
        (:`else`)))))

(fn `UserConstructionScript`)