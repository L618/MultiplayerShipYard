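; MainGI is the game instance Blueprint that manages multiplayer sessions for hosting, quick play and disconnecting.
; Hosting creates a LAN or online session, flags the instance as hoster and opens the chosen level with the given options.
; Quick play joins the first session found, without filtering.
; Destroying a session can return the player to MainMenu with a disconnect message, while travel, network and session failures print on-screen debug text.
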(event `self.HandleTravelError`
  (params (FailureType :type "ETravelFailure Enum" :default "NoLevel"))
  ;[1 0 0] Travel Error
  (`KismetSystemLibrary.PrintString` (`|GetEnumeratorNameAsString` FailureType) true true (struct :`G` 0.66 :`B` 1.0 :`A` 1.0) 22.0))

(event `E_HostGame`
  (params (PublicConnections :type Integer) (bUseLAN :type Boolean) (LevelName :type Name) (Options :type String))
  ;[1 1 1] Host Game
  (`CreateSessionCallbackProxy.CreateSession` (`GameplayStatics.GetPlayerController` 0) PublicConnections bUseLAN
    (:`OnSuccess`
      (set `self.IsHoster` true)
      (`GameplayStatics.OpenLevel` LevelName true Options))
    (:`OnFailure`
      (`KismetSystemLibrary.PrintString` "SESSION CREATION ERROR" true true (struct :`G` 0.66 :`B` 1.0 :`A` 1.0) 22.0))))

(event `self.HandleNetworkError`
  (params (FailureType :type "ENetworkFailure Enum" :default "NetDriverAlreadyExists") (bIsServer :type Boolean))
  ;[1 0 0] Network Error
  (`KismetSystemLibrary.PrintString` (`|GetEnumeratorNameAsString` FailureType) true true (struct :`G` 0.66 :`B` 1.0 :`A` 1.0) 22.0))

(event `E_QuickPlay`
  (params (bUseLAN :type Boolean))
  ;[1 1 1] Quick Play
  (bind _results (`FindSessionsCallbackProxy.FindSessions` (`GameplayStatics.GetPlayerController` 0) 100 bUseLAN)
    (:`OnSuccess`
      (`JoinSessionCallbackProxy.JoinSession` (`GameplayStatics.GetPlayerController` 0) (`|GetArrayItem` _results)
        (:`OnFailure`
          (`KismetSystemLibrary.PrintString` " QUICK PLAY SESSION COONECTION ERROR" true true (struct :`G` 0.66 :`B` 1.0 :`A` 1.0) 22.0))))
    (:`OnFailure`
      (`KismetSystemLibrary.PrintString` " QUICK PLAY - Find session FAIL" true true (struct :`G` 0.66 :`B` 1.0 :`A` 1.0) 22.0))))

(event `E_DestroySessionCaller`
  (params (PlayerController :type "PlayerController Object Reference") (ReturnToMain_Menu :type Boolean))
  (`DestroySessionCallbackProxy.DestroySession` PlayerController
    (:`then`
      (if ReturnToMain_Menu
        (`GameplayStatics.OpenLevel` "MainMenu")
        (`KismetSystemLibrary.PrintString` "You have been disconnected from the server" true true (struct :`R` 1.0 :`A` 1.0) 22.0)))))