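; Player character for the BR mode, handling team appearance, teammate name tags and point damage.
; Shortly after BeginPlay, in multi-team games, it applies the team material and shows team-colored names on non-local teammates.
; Point damage is gated by game state, death and the friendly-fire setting; headshots zero health.
; Health is mirrored to the PlayerState, and death is reported with victim, killer, damage causer and headshot flag.
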(event `self.ReceiveBeginPlay`
  (`parent.ReceiveBeginPlay`)
  (`KismetSystemLibrary.Delay` 2.0)
  (`|ExecutionSequence`
    (:`then_0`
      (if (> (`/Game/RPMSF/Blueprints/Kernel/MainGI.TeamsQty` (`/Game/RPMSF/Blueprints/Kernel/Helpers.H_GetMainGI`)) 1)
        (`self.E_SetTeamMaterial` (`/Game/RPMSF/Blueprints/Kernel/CoreClasses/Core_PS.Team` (cast `/Game/RPMSF/Blueprints/Kernel/CoreClasses/Core_PS` (`self.PlayerState`) :!pure true)))))
    (:`then_1`
      (if (not (`self.IsLocallyControlled`))
        (`self.E_ShowNameForTeammate`)))))

(event `E_ShowNameForTeammate`
  (bind _playername (`self.PlayerName`))
  ;[1 1 1] Show player name for teammates
  (if (> (`/Game/RPMSF/Blueprints/Kernel/MainGI.TeamsQty` (`/Game/RPMSF/Blueprints/Kernel/Helpers.H_GetMainGI`)) 1)
    (bind _asbr_ps (cast `/Game/RPMSF/Blueprints/CustomGameModes/BattleRoyale/BR_PS` (`self.PlayerState`)))
    (bind _team (`/Game/RPMSF/Blueprints/Kernel/CoreClasses/Core_PS.Team` _asbr_ps))
    (if (== _team (`/Game/RPMSF/Blueprints/Kernel/CoreClasses/Core_PS.Team` (cast `/Game/RPMSF/Blueprints/CustomGameModes/BattleRoyale/BR_PS` (`Controller.PlayerState` (`GameplayStatics.GetPlayerController` 0)) :!pure true)))
      (`SceneComponent.SetVisibility` _playername true false)
      (`TextRenderComponent.K2_SetText` _playername (`KismetTextLibrary.Conv_StringToText` (`PlayerState.GetPlayerName` (`self.PlayerState`))))
      (`TextRenderComponent.SetTextRenderColor` _playername (`KismetMathLibrary.Conv_LinearColorToColor` (`/Game/RPMSF/Blueprints/Kernel/Helpers.H_GetTeamDataFromDB` _team))))))

(event `self.ReceivePointDamage`
  (params (Damage :type "Float (single-precision)") (DamageType :type "DamageType Object Reference") (HitLocation :type "Vector Structure") (HitNormal :type "Vector Structure") (HitComponent :type "PrimitiveComponent Object Reference") (BoneName :type Name) (ShotFromDirection :type "Vector Structure") (InstigatedBy :type "Controller Object Reference") (DamageCauser :type "Actor Object Reference") (HitInfo :type "HitResult Structure (by ref)"))
  (bind _isheadshot (`self.FS_IsHeadShot` BoneName))
  (bind _playerstate (`Controller.PlayerState` InstigatedBy))
  (bind _asbr_ps (cast `/Game/RPMSF/Blueprints/CustomGameModes/BattleRoyale/BR_PS` (`self.PlayerState`) :!pure true))
  ;[0.8646 0 0.1981] APPLY DAMAGE
  (if (`self.FS_CanApplyDamage` _playerstate)
    (`self.D_DamageTaken`)
    (if _isheadshot
      (set `self.Health` 0.0)
      (set `/Game/RPMSF/Blueprints/CustomGameModes/BattleRoyale/BR_PS.Health` 0.0 _asbr_ps)
      (else
        (bind _output_get (set `self.Health` (- (`self.Health`) Damage)))
        (set `/Game/RPMSF/Blueprints/CustomGameModes/BattleRoyale/BR_PS.Health` _output_get _asbr_ps)))
    (if (<= _output_get 0.0)
      (set `self.IsDead` true)
      (`/Game/RPMSF/Blueprints/Kernel_Character/Interfaces/I_CoreCharacter.IE_Death` (`self.PlayerState`) _playerstate DamageCauser _isheadshot))))

(fn `FS_CanApplyDamage`
  (params (ShooterPS :type "PlayerState Object Reference"))
  (returns (ApplyDamage :type Boolean))
  (locals (isFriendlyFire :type Boolean))
  (bind _globalstate (`/Game/RPMSF/Blueprints/Kernel/CoreClasses/Core_GS.GlobalState` (`/Game/RPMSF/Blueprints/Kernel/Helpers.H_GetCoreGS`)))
  (bind _globalstate_2 (`/Game/RPMSF/Blueprints/Kernel/CoreClasses/Core_GS.GlobalState` (`/Game/RPMSF/Blueprints/Kernel/Helpers.H_GetCoreGS`)))
  (`|ExecutionSequence`
    (:`then_0`
      (bind _ascore_ps (cast `/Game/RPMSF/Blueprints/Kernel/CoreClasses/Core_PS` ShooterPS)
        (:`then`
          (bind _ascore_ps_2 (cast `/Game/RPMSF/Blueprints/Kernel/CoreClasses/Core_PS` (`self.PlayerState`))
            (:`then`
              (set `local.isFriendlyFire` (== (`/Game/RPMSF/Blueprints/Kernel/CoreClasses/Core_PS.Team` _ascore_ps_2) (`/Game/RPMSF/Blueprints/Kernel/CoreClasses/Core_PS.Team` _ascore_ps))))
            (:`CastFailed`
              (set `local.isFriendlyFire` false))))
        (:`CastFailed`
          (set `local.isFriendlyFire` false))))
    (:`then_1`
      (if (`/Game/RPMSF/Blueprints/Kernel/CoreClasses/Core_GM.isFriendlyFireAllowed` (`/Game/RPMSF/Blueprints/Kernel/Helpers.H_GetCoreGM`))
        (return (and (not (`self.IsDead`)) (or (`|EnumEquality` _globalstate_2 "NewEnumerator16") (`|EnumEquality` _globalstate_2 "NewEnumerator17"))))
        (else
          (return (and (or (`|EnumEquality` _globalstate "NewEnumerator16") (`|EnumEquality` _globalstate "NewEnumerator17")) (not (`local.IsFriendlyFire`)) (not (`self.IsDead`)))))))))

(fn `UserConstructionScript`
  (`parent.UserConstructionScript`))